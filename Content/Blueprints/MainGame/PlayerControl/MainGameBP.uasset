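; MainGameBP drives the main game's money display and its lose condition.
; On BeginPlay it gathers all ComputerSpot actors as computer spawn points and creates the MainGameUI widget on screen.
; Each Tick writes PlayerMoney into the widget's text block and opens the MainMenu level once money drops to zero or below.
; An unconnected branch that would create a UIComputerBuilder widget never runs.
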(event EventBeginPlay
  (bind _outactors (Actor|GetAllActorsOfClass "/Game/Blueprints/MainGame/ComputerStand/ComputerSpot.ComputerSpot_C"))
  (Variables|Default|SetComputerSpawnPoints _outactors)
  (bind _returnvalue (UserInterface|CreateWidget "/Game/Blueprints/MainGame/MainGameUI.MainGameUI_C"))
  (UserInterface|Viewport|AddtoViewport _returnvalue 0)
  (Variables|Default|SetMainGameUI _returnvalue))

(event EventTick
  (params (DeltaSeconds :type Float%20%28single-precision%29))
  (bind _asmain_game_ui (Utilities|Casting|CastToMainGameUI (Variables|Default|GetMainGameUI)))
  (Rendering|Components|TextRender|SetText (Variables|/Game/Blueprints/MainGame/MainGameUI.MainGameUI_C|GetTextBlock_219 _asmain_game_ui) (Utilities|Text|ToText(Float) (Variables|Default|GetPlayerMoney) "HalfToEven"))
  (if (<= (Variables|Default|GetPlayerMoney) 0.0)
    (Game|OpenLevel(byName) "MainMenu")))

(fn ConstructionScript)