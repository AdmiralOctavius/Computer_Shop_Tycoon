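; Main game controller that handles mouse-cursor interaction with world objects and exits to the main menu.
; Each tick it traces from the deprojected mouse position along the visibility channel and stores the hit location in BroadcastCursorLocation.
; Interact repeats the trace, sending off-click to LastObject and click to a newly hit actor, or re-clicking the same one.
; Exit opens the MainMenu level, while a QuitGame node sits unconnected.
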(event EventBeginPlay)

(event EventTick
  (params (DeltaSeconds :type Float%20%28single-precision%29))
  (bind (_worldlocation _worlddirection) (Game|Player|ConvertMouseLocationToWorldSpace))
  (bind _outhit (Collision|LineTraceByChannel _worldlocation (+ _worldlocation (+ (* _worlddirection (Variables|Default|GetClickRange)) _worlddirection)) "TraceTypeQuery1" false 0 "None"))
  (Variables|Default|SetbroadcastCursorLocation (.location _outhit)))

(event Input|ActionEvents|InputActionExit
  (params (Key :type Key%20Structure))
  (:Pressed
    (Game|OpenLevel(byName) "MainMenu")))

(event Input|ActionEvents|InputActionInteract
  (params (Key :type Key%20Structure))
  (bind (_worldlocation _worlddirection) (Game|Player|ConvertMouseLocationToWorldSpace))
  (:Pressed
    (bind _outhit (Collision|LineTraceByChannel _worldlocation (+ _worldlocation (+ (* _worlddirection (Variables|Default|GetClickRange)) _worlddirection)) "TraceTypeQuery1" false 0 "ForDuration"))
    (if (!= (.hitactor _outhit) (Variables|Default|GetLastObject))
      (Class|SelectableInterface|OffClick(Message) (Variables|Default|GetLastObject))
      (Class|SelectableInterface|OnClickedItem(Message) (.hitactor _outhit))
      (Variables|Default|SetLastObject (.hitactor _outhit))
      (else
        (Class|SelectableInterface|OnClickedItem(Message) (Variables|Default|GetLastObject))))))

(fn ConstructionScript)